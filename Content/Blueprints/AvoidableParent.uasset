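; Parent Blueprint for obstacles that scroll along negative X at a fixed per-tick step and kill the player on contact.
; Overlaps are identified by object name: the reset trigger returns the actor to InitialPosition with a random height.
; A player hit also repositions it, plays a slap sound, pauses the game, then opens MainMenu after a delay.
; The actor is set tickable when paused to support this death sequence.
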(event `self.ReceiveBeginPlay`
  ;[1 1 1] Set Tickable on BeginPlay to allow pausing when dying
  (`self.SetTickableWhenPaused` true))

(event `self.ReceiveActorBeginOverlap`
  (params (OtherActor :type "Actor Object Reference"))
  ;[1 1 1] Check if Overlap was with PlayerCharacter
  (if (`KismetStringLibrary.EqualEqual_StrStr` (`KismetSystemLibrary.GetObjectName` OtherActor) (`KismetSystemLibrary.GetObjectName` (`GameplayStatics.GetPlayerCharacter` 0)))
    ;[1 1 1] PlayerCharacter was hit, play the slap sound
    (`GameplayStatics.PlaySound2D` "/Game/Sounds/Slap-SoundMaster13-49669815.Slap-SoundMaster13-49669815" 0.5 1.0 0.0 null null)
    ;[1 1 1] SetActionLocation to Initial Position, with randomized Z value
    (`self.K2_SetActorLocation` (`KismetMathLibrary.MakeVector` (.x (`self.InitialPosition`)) (.y (`self.InitialPosition`)) (`KismetMathLibrary.RandomFloatInRange` (.z (`self.InitialPosition`)) 500.0)))
    ;[1 1 1] Player has died, go to Main Menu
    (`KismetSystemLibrary.PrintText` "You died.")
    (`GameplayStatics.SetGamePaused` true)
    (`KismetSystemLibrary.Delay` 2.0)
    (`GameplayStatics.OpenLevel` "MainMenu")
    (else
      ;[1 1 1] If Overlap wasn't PlayerCharacter, check if we hit the reset trigger
      (if (`KismetStringLibrary.EqualEqual_StrStr` (`KismetSystemLibrary.GetObjectName` OtherActor) "ResetMoneybagTrigger")
        ;[1 1 1] SetActorLocation to Initial Position, with randomized Z value
        (`self.K2_SetActorLocation` (`KismetMathLibrary.MakeVector` (.x (`self.InitialPosition`)) (.y (`self.InitialPosition`)) (`KismetMathLibrary.RandomFloatInRange` (.z (`self.InitialPosition`)) 300.0)))))))

(event `self.ReceiveTick`
  (params (DeltaSeconds :type "Float (single-precision)"))
  ;[1 1 1] Move the Actor on Event Tick
  (`self.K2_AddActorWorldOffset` (-5.0 0.0 0.0)))

(fn `UserConstructionScript`)